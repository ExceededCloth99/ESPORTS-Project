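; Game Instance that acts as the central hub for the game's menus, pause toggle and single or multiplayer entry.
; Events create the title, start, host/find and pause widgets, switching input mode and cursor, and also open the single-player map, join or destroy sessions, and quit.
; Per-menu state-check events read button focus and restyle the current selection with brushes built in Init, with most restoring lost focus for keyboard-style navigation.
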(event Custom|StartMainMenu
  (bind _returnvalue (Game|GetPlayerController 0))
  ;[1 1 1] Load Start Menu
  (bind _returnvalue_2 (UserInterface|CreateWidget "/Game/UserInterface/StartMenu.StartMenu_C" _returnvalue))
  (bind _output_get (Variables|Default|SetStartMenuRef _returnvalue_2))
  (UserInterface|Viewport|AddtoViewport _output_get 1)
  (Input|SetInputModeUIOnly _returnvalue (Variables|/Game/UserInterface/StartMenu.StartMenu_C|GetSingle_btn _returnvalue_2) "DoNotLock")
  (Variables|/Script/Engine.PlayerController|SetbShowMouseCursor _returnvalue true))

(event Custom|ExitGame
  ;[1 1 1] Quit Game
  (Game|QuitGame 0 "Quit" false))

(event Custom|JoinToSelectedServer
  (params (Search%20Result :type Blueprint%20Session%20Result%20Structure))
  (|JoinSession (Game|GetPlayerController 0) Search%20Result))

(event Custom|LoadFindMenu
  (bind _returnvalue (UserInterface|CreateWidget "/Game/UserInterface/FindMenu.FindMenu_C" (Game|GetPlayerController 0)))
  (bind _output_get (Variables|Default|SetFindMenuRef _returnvalue))
  (UserInterface|Viewport|AddtoViewport _output_get 0))

(event Custom|DestroyAllSessions
  ;[1 1 1] Destroy All Sessions
  (|DestroySession (Game|GetPlayerController 0)
    (:OnSuccess
      (Development|PrintString "Session Destroyed"))
    (:OnFailure
      (Development|PrintString "Session Not Destroyed"))))

(event Custom|FindMenuStateCheck
  (bind _findmenuref (Variables|Default|GetFindMenuRef))
  (bind _findmenuref_2 (Variables|Default|GetFindMenuRef))
  (bind _unselectedstyle (Variables|Default|GetUnselectedStyle))
  (bind _findmenuref_3 (Variables|Default|GetFindMenuRef))
  (bind _buttonstyle (Utilities|Struct|MakeButtonStyle _unselectedstyle "(ImageSize=(X=32.000000,Y=32.000000),Margin=(Left=0.000000,Top=0.000000,Right=0.000000,Bottom=0.000000),Tint=(R=1.000000,G=1.000000,B=1.000000,A=1.000000),TintColor=(SpecifiedColor=(R=1.000000,G=1.000000,B=1.000000,A=1.000000),ColorUseRule=UseColor_Specified),ResourceObject=None,ResourceName=\"\",UVRegion=(Min=(X=0.000000,Y=0.000000),Max=(X=0.000000,Y=0.000000),bIsValid=0),DrawAs=Image,Tiling=NoTile,Mirroring=NoMirror,ImageType=NoImage,bIsDynamicallyLoaded=False,bHasUObject=False)"))
  (bind _search_btn (Variables|/Game/UserInterface/FindMenu.FindMenu_C|GetSearch_btn _findmenuref_2))
  (bind _hostfind_btn (Variables|/Game/UserInterface/FindMenu.FindMenu_C|GetHostFind_btn _findmenuref))
  ;[1 1 1] Find State Check
  (if (Math|Boolean|Equal(Boolean) (Class|Widget|HasAnyUserFocus _search_btn) true)
    (Variables|Default|SetCurrentSelection _search_btn)
    (elif (Math|Boolean|Equal(Boolean) (Class|Widget|HasAnyUserFocus _hostfind_btn) true)
      (Variables|Default|SetCurrentSelection _hostfind_btn)))
  (Variables|/Script/UMG.Button|SetWidgetStyle (Variables|/Game/UserInterface/FindMenu.FindMenu_C|GetHostFind_btn _findmenuref_3) _buttonstyle)
  (Variables|/Script/UMG.Button|SetWidgetStyle (Variables|/Game/UserInterface/FindMenu.FindMenu_C|GetSearch_btn _findmenuref_3) _buttonstyle)
  (Variables|/Script/UMG.Button|SetWidgetStyle (Variables|Default|GetCurrentSelection) (Utilities|Struct|MakeButtonStyle (Variables|Default|GetSelectedStyle) "(ImageSize=(X=32.000000,Y=32.000000),Margin=(Left=0.000000,Top=0.000000,Right=0.000000,Bottom=0.000000),Tint=(R=1.000000,G=1.000000,B=1.000000,A=1.000000),TintColor=(SpecifiedColor=(R=1.000000,G=1.000000,B=1.000000,A=1.000000),ColorUseRule=UseColor_Specified),ResourceObject=None,ResourceName=\"\",UVRegion=(Min=(X=0.000000,Y=0.000000),Max=(X=0.000000,Y=0.000000),bIsValid=0),DrawAs=Image,Tiling=NoTile,Mirroring=NoMirror,ImageType=NoImage,bIsDynamicallyLoaded=False,bHasUObject=False)")))

(event Custom|SetFirstServer
  (params (FirstServer :type Button%20Object%20Reference))
  (Utilities|IsValid (Variables|Default|GetFirstServer)
    (:Is%20Not%20Valid
      (Variables|Default|SetFirstServer FirstServer)
      (Variables|Default|SetHasSetServerFocus? true))))

(event Custom|FocusOnFirstServer
  (Class|Widget|SetUserFocus (Variables|Default|GetFirstServer) (Game|GetPlayerController 0)))

(event Custom|SinglePlayer
  (bind _startmenuref (Variables|Default|GetStartMenuRef))
  (bind _fadetoblack (Variables|/Game/UserInterface/StartMenu.StartMenu_C|GetFadeToBlack _startmenuref))
  ;[1 1 1] Start Single Player
  (UserInterface|Animation|PlayAnimation _fadetoblack (Variables|/Game/UserInterface/FadeToBlack.FadeToBlack_C|GetFadeIn _fadetoblack) 0.0 1 "Forward" 1.0)
  (Utilities|FlowControl|Delay 1.0)
  (Game|OpenLevel(byName) "ThirdPersonExampleMap")
  (Input|SetInputModeGameOnly (Game|GetPlayerController 0)))

(event Custom|MultiPlayer
  (bind _returnvalue (Game|GetPlayerController 0))
  ;[1 1 1] Start MultiPlayer Game
  (bind _returnvalue_2 (UserInterface|CreateWidget "/Game/UserInterface/HostFindMenu.HostFindMenu_C" _returnvalue))
  (bind _output_get (Variables|Default|SetHostFindRef _returnvalue_2))
  (UserInterface|Viewport|AddtoViewport _output_get 1)
  (Input|SetInputModeUIOnly _returnvalue (Variables|/Game/UserInterface/HostFindMenu.HostFindMenu_C|GetHostGame_btn _returnvalue_2) "DoNotLock")
  (Variables|/Script/Engine.PlayerController|SetbShowMouseCursor _returnvalue true))

(event Custom|SingleMultiMenuStateCheck
  (bind _startmenuref (Variables|Default|GetStartMenuRef))
  (bind _unselectedstyle (Variables|Default|GetUnselectedStyle))
  (bind _buttonstyle (Utilities|Struct|MakeButtonStyle _unselectedstyle "(ImageSize=(X=32.000000,Y=32.000000),Margin=(Left=0.000000,Top=0.000000,Right=0.000000,Bottom=0.000000),Tint=(R=1.000000,G=1.000000,B=1.000000,A=1.000000),TintColor=(SpecifiedColor=(R=1.000000,G=1.000000,B=1.000000,A=1.000000),ColorUseRule=UseColor_Specified),ResourceObject=None,ResourceName=\"\",UVRegion=(Min=(X=0.000000,Y=0.000000),Max=(X=0.000000,Y=0.000000),bIsValid=0),DrawAs=Image,Tiling=NoTile,Mirroring=NoMirror,ImageType=NoImage,bIsDynamicallyLoaded=False,bHasUObject=False)"))
  ;[1 1 1] Single Multi State Check
  (Variables|Default|SetCurrentSelection (Variables|/Game/UserInterface/StartMenu.StartMenu_C|GetSingle_btn (Variables|Default|GetStartMenuRef)))
  (if (Math|Boolean|Equal(Boolean) (Class|Widget|HasAnyUserFocus (Variables|/Game/UserInterface/StartMenu.StartMenu_C|GetSingle_btn (Variables|Default|GetStartMenuRef))) true)
    (Variables|Default|SetCurrentSelection (Variables|/Game/UserInterface/StartMenu.StartMenu_C|GetSingle_btn (Variables|Default|GetStartMenuRef)))
    (Variables|/Script/UMG.Button|SetWidgetStyle (Variables|/Game/UserInterface/StartMenu.StartMenu_C|GetSingle_btn _startmenuref) _buttonstyle :!label _label)
    (Variables|/Script/UMG.Button|SetWidgetStyle (Variables|/Game/UserInterface/StartMenu.StartMenu_C|GetMulti_btn _startmenuref) _buttonstyle)
    (Variables|/Script/UMG.Button|SetWidgetStyle (Variables|/Game/UserInterface/StartMenu.StartMenu_C|GetExit_btn _startmenuref) _buttonstyle)
    (Variables|/Script/UMG.Button|SetWidgetStyle (Variables|Default|GetCurrentSelection) (Utilities|Struct|MakeButtonStyle (Variables|Default|GetSelectedStyle) "(ImageSize=(X=32.000000,Y=32.000000),Margin=(Left=0.000000,Top=0.000000,Right=0.000000,Bottom=0.000000),Tint=(R=1.000000,G=1.000000,B=1.000000,A=1.000000),TintColor=(SpecifiedColor=(R=1.000000,G=1.000000,B=1.000000,A=1.000000),ColorUseRule=UseColor_Specified),ResourceObject=None,ResourceName=\"\",UVRegion=(Min=(X=0.000000,Y=0.000000),Max=(X=0.000000,Y=0.000000),bIsValid=0),DrawAs=Image,Tiling=NoTile,Mirroring=NoMirror,ImageType=NoImage,bIsDynamicallyLoaded=False,bHasUObject=False)"))
    (elif (Math|Boolean|Equal(Boolean) (Class|Widget|HasKeyboardFocus (Variables|/Game/UserInterface/StartMenu.StartMenu_C|GetMulti_btn (Variables|Default|GetStartMenuRef))) true)
      (Variables|Default|SetCurrentSelection (Variables|/Game/UserInterface/StartMenu.StartMenu_C|GetMulti_btn (Variables|Default|GetStartMenuRef)))
      (goto _label)
      (elif (Math|Boolean|Equal(Boolean) (Class|Widget|HasKeyboardFocus (Variables|/Game/UserInterface/StartMenu.StartMenu_C|GetExit_btn (Variables|Default|GetStartMenuRef))) true)
        (Variables|Default|SetCurrentSelection (Variables|/Game/UserInterface/StartMenu.StartMenu_C|GetExit_btn (Variables|Default|GetStartMenuRef)))
        (goto _label)
        (else
          (Class|Widget|SetUserFocus (Variables|Default|GetCurrentSelection) (Game|GetPlayerController 0)))))))

(event Custom|LoadMainMenu
  (bind _returnvalue (Game|GetPlayerController 0))
  ;[1 1 1] Load Main Menu / Title Sequence
  (bind _returnvalue_2 (UserInterface|CreateWidget "/Game/UserInterface/MainMenu.MainMenu_C" _returnvalue))
  (bind _output_get (Variables|Default|SetMain_Menu _returnvalue_2))
  (UserInterface|Viewport|AddtoViewport _output_get 0)
  (Input|SetInputModeUIOnly _returnvalue _output_get "DoNotLock")
  (Variables|/Script/Engine.PlayerController|SetbShowMouseCursor _returnvalue true))

(event Custom|PauseGame
  (bind _returnvalue (Game|GetPlayerController 0))
  ;[1 1 1] Pause Game
  (if (Variables|Default|GetIsPaused)
    (Widget|RemovefromParent (stale _returnvalue_2))
    (Variables|/Script/Engine.PlayerController|SetbShowMouseCursor _returnvalue false)
    (Game|SetGamePaused false)
    (Input|SetInputModeGameOnly _returnvalue)
    (Variables|Default|SetIsPaused false)
    (else
      (bind _returnvalue_2 (UserInterface|CreateWidget "/Game/UserInterface/PauseMenu.PauseMenu_C" _returnvalue))
      (bind _output_get (Variables|Default|SetPauseMenuRef _returnvalue_2))
      (UserInterface|Viewport|AddtoViewport _output_get 0)
      (Variables|/Script/Engine.PlayerController|SetbShowMouseCursor _returnvalue true)
      (Game|SetGamePaused true)
      (Input|SetInputModeGameandUI _returnvalue (Variables|/Game/UserInterface/PauseMenu.PauseMenu_C|GetMainMenu_btn _returnvalue_2) "DoNotLock" true)
      (Variables|Default|SetIsPaused true))))

(event Custom|PauseMenuStateCheck
  (bind _pausemenuref (Variables|Default|GetPauseMenuRef))
  (bind _pausemenuref_2 (Variables|Default|GetPauseMenuRef))
  (bind _unselectedstyle (Variables|Default|GetUnselectedStyle))
  (bind _pausemenuref_3 (Variables|Default|GetPauseMenuRef))
  (bind _buttonstyle (Utilities|Struct|MakeButtonStyle _unselectedstyle "(ImageSize=(X=32.000000,Y=32.000000),Margin=(Left=0.000000,Top=0.000000,Right=0.000000,Bottom=0.000000),Tint=(R=1.000000,G=1.000000,B=1.000000,A=1.000000),TintColor=(SpecifiedColor=(R=1.000000,G=1.000000,B=1.000000,A=1.000000),ColorUseRule=UseColor_Specified),ResourceObject=None,ResourceName=\"\",UVRegion=(Min=(X=0.000000,Y=0.000000),Max=(X=0.000000,Y=0.000000),bIsValid=0),DrawAs=Image,Tiling=NoTile,Mirroring=NoMirror,ImageType=NoImage,bIsDynamicallyLoaded=False,bHasUObject=False)"))
  (bind _mainmenu_btn (Variables|/Game/UserInterface/PauseMenu.PauseMenu_C|GetMainMenu_btn _pausemenuref))
  (bind _resume_btn (Variables|/Game/UserInterface/PauseMenu.PauseMenu_C|GetResume_btn _pausemenuref_3))
  ;[1 1 1] Pause Menu State Check
  (if (Math|Boolean|Equal(Boolean) (Class|Widget|HasAnyUserFocus _mainmenu_btn) true)
    (Variables|Default|SetCurrentSelection _mainmenu_btn)
    (Variables|/Script/UMG.Button|SetWidgetStyle (Variables|/Game/UserInterface/PauseMenu.PauseMenu_C|GetResume_btn _pausemenuref_2) _buttonstyle :!label _label)
    (Variables|/Script/UMG.Button|SetWidgetStyle (Variables|/Game/UserInterface/PauseMenu.PauseMenu_C|GetMainMenu_btn _pausemenuref_2) _buttonstyle)
    (Variables|/Script/UMG.Button|SetWidgetStyle (Variables|Default|GetCurrentSelection) (Utilities|Struct|MakeButtonStyle (Variables|Default|GetSelectedStyle) "(ImageSize=(X=32.000000,Y=32.000000),Margin=(Left=0.000000,Top=0.000000,Right=0.000000,Bottom=0.000000),Tint=(R=1.000000,G=1.000000,B=1.000000,A=1.000000),TintColor=(SpecifiedColor=(R=1.000000,G=1.000000,B=1.000000,A=1.000000),ColorUseRule=UseColor_Specified),ResourceObject=None,ResourceName=\"\",UVRegion=(Min=(X=0.000000,Y=0.000000),Max=(X=0.000000,Y=0.000000),bIsValid=0),DrawAs=Image,Tiling=NoTile,Mirroring=NoMirror,ImageType=NoImage,bIsDynamicallyLoaded=False,bHasUObject=False)"))
    (elif (Math|Boolean|Equal(Boolean) (Class|Widget|HasAnyUserFocus _resume_btn) true)
      (Variables|Default|SetCurrentSelection _resume_btn)
      (goto _label)
      (else
        (Class|Widget|SetUserFocus (Variables|Default|GetCurrentSelection) (Game|GetPlayerController 0))))))

(event Custom|HostFindStateCheck
  (bind _hostfindref (Variables|Default|GetHostFindRef))
  (bind _hostfindref_2 (Variables|Default|GetHostFindRef))
  (bind _hostfindref_3 (Variables|Default|GetHostFindRef))
  (bind _unselectedstyle (Variables|Default|GetUnselectedStyle))
  (bind _hostfindref_4 (Variables|Default|GetHostFindRef))
  (bind _buttonstyle (Utilities|Struct|MakeButtonStyle _unselectedstyle "(ImageSize=(X=32.000000,Y=32.000000),Margin=(Left=0.000000,Top=0.000000,Right=0.000000,Bottom=0.000000),Tint=(R=1.000000,G=1.000000,B=1.000000,A=1.000000),TintColor=(SpecifiedColor=(R=1.000000,G=1.000000,B=1.000000,A=1.000000),ColorUseRule=UseColor_Specified),ResourceObject=None,ResourceName=\"\",UVRegion=(Min=(X=0.000000,Y=0.000000),Max=(X=0.000000,Y=0.000000),bIsValid=0),DrawAs=Image,Tiling=NoTile,Mirroring=NoMirror,ImageType=NoImage,bIsDynamicallyLoaded=False,bHasUObject=False)"))
  (bind _hostgame_btn (Variables|/Game/UserInterface/HostFindMenu.HostFindMenu_C|GetHostGame_btn _hostfindref))
  (bind _findgames_btn (Variables|/Game/UserInterface/HostFindMenu.HostFindMenu_C|GetFindGames_btn _hostfindref_3))
  (bind _mainmenu_btn (Variables|/Game/UserInterface/HostFindMenu.HostFindMenu_C|GetMainMenu_btn _hostfindref_2))
  ;[1 1 1] HostFind State Check
  (if (Math|Boolean|Equal(Boolean) (Class|Widget|HasAnyUserFocus _hostgame_btn) true)
    (Variables|Default|SetCurrentSelection _hostgame_btn)
    (Variables|/Script/UMG.Button|SetWidgetStyle (Variables|/Game/UserInterface/HostFindMenu.HostFindMenu_C|GetFindGames_btn _hostfindref_4) _buttonstyle :!label _label)
    (Variables|/Script/UMG.Button|SetWidgetStyle (Variables|/Game/UserInterface/HostFindMenu.HostFindMenu_C|GetHostGame_btn _hostfindref_4) _buttonstyle)
    (Variables|/Script/UMG.Button|SetWidgetStyle (Variables|/Game/UserInterface/HostFindMenu.HostFindMenu_C|GetMainMenu_btn _hostfindref_4) _buttonstyle)
    (Variables|/Script/UMG.Button|SetWidgetStyle (Variables|Default|GetCurrentSelection) (Utilities|Struct|MakeButtonStyle (Variables|Default|GetSelectedStyle) "(ImageSize=(X=32.000000,Y=32.000000),Margin=(Left=0.000000,Top=0.000000,Right=0.000000,Bottom=0.000000),Tint=(R=1.000000,G=1.000000,B=1.000000,A=1.000000),TintColor=(SpecifiedColor=(R=1.000000,G=1.000000,B=1.000000,A=1.000000),ColorUseRule=UseColor_Specified),ResourceObject=None,ResourceName=\"\",UVRegion=(Min=(X=0.000000,Y=0.000000),Max=(X=0.000000,Y=0.000000),bIsValid=0),DrawAs=Image,Tiling=NoTile,Mirroring=NoMirror,ImageType=NoImage,bIsDynamicallyLoaded=False,bHasUObject=False)"))
    (elif (Math|Boolean|Equal(Boolean) (Class|Widget|HasAnyUserFocus _findgames_btn) true)
      (Variables|Default|SetCurrentSelection _findgames_btn)
      (goto _label)
      (elif (Math|Boolean|Equal(Boolean) (Class|Widget|HasAnyUserFocus _mainmenu_btn) true)
        (Variables|Default|SetCurrentSelection _mainmenu_btn)
        (goto _label)
        (else
          (Class|Widget|SetUserFocus (Variables|Default|GetCurrentSelection) (Game|GetPlayerController 0)))))))

(event Custom|LoadHostMenu
  (bind _returnvalue (Game|GetPlayerController 0))
  (bind _returnvalue_2 (UserInterface|CreateWidget "/Game/UserInterface/HostMenu.HostMenu_C" _returnvalue))
  (bind _output_get (Variables|Default|SetHostMenuRef _returnvalue_2))
  (UserInterface|Viewport|AddtoViewport _output_get 0)
  (Input|SetInputModeUIOnly _returnvalue (Variables|/Game/UserInterface/HostMenu.HostMenu_C|GetIncrease _returnvalue_2) "DoNotLock")
  (Variables|/Script/Engine.PlayerController|SetbShowMouseCursor _returnvalue true))

(event EventInit
  ;[1 1 1] Set button Style
  (Variables|Default|SetSelectedStyle (Utilities|Struct|MakeSlateBrush "(X=32.000000,Y=32.000000)" "(Left=0.000000,Top=0.000000,Right=0.000000,Bottom=0.000000)" (Utilities|Struct|MakeSlateColor "(R=1.000000,G=0.000000,B=0.000000,A=1.000000)" "UseColor_Foreground") 0 "Image" "NoTile" "NoMirror"))
  (Variables|Default|SetUnselectedStyle (Utilities|Struct|MakeSlateBrush "(X=32.000000,Y=32.000000)" "(Left=0.000000,Top=0.000000,Right=0.000000,Bottom=0.000000)" (Utilities|Struct|MakeSlateColor "(R=1.000000,G=1.000000,B=1.000000,A=0.000000)") 0 "Image" "NoTile" "NoMirror")))