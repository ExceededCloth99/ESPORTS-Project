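; DropGate is a gate actor that moves its mesh vertically to close when CloseGate is called.
; Its trigger volume registers the gate with an overlapping ThirdPersonCharacter and toggles that character's interaction widget, clearing both on exit.
; CloseGate passes a DoOnce with no reset, then plays the GateClose timeline to drive the mesh's relative Z.
; A separate ClosePlatform event reverses the same timeline.
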(event OnComponentBeginOverlap(TriggerVolume)
  (params (OverlappedComponent :type Primitive%20Component%20Object%20Reference) (OtherActor :type Actor%20Object%20Reference) (OtherComp :type Primitive%20Component%20Object%20Reference) (OtherBodyIndex :type Integer) (bFromSweep :type Boolean) (SweepResult :type Hit%20Result%20Structure%20%28by%20ref%29))
  ;[1 1 1] Check Gate Proximity#
  (bind _asthird_person_character (Utilities|Casting|CastToThirdPersonCharacter OtherActor))
  (if (stale _bsuccess)
    (Default|InteractwithGate _asthird_person_character self true)
    (Variables|/Game/ThirdPersonBP/Blueprints/ThirdPersonCharacter.ThirdPersonCharacter_C|SetWidgetVisible _asthird_person_character true)))

(event OnComponentEndOverlap(TriggerVolume)
  (params (OverlappedComponent :type Primitive%20Component%20Object%20Reference) (OtherActor :type Actor%20Object%20Reference) (OtherComp :type Primitive%20Component%20Object%20Reference) (OtherBodyIndex :type Integer))
  ;[1 1 1] Check Gate Proximity#
  (bind _asthird_person_character (Utilities|Casting|CastToThirdPersonCharacter OtherActor))
  (if (stale _bsuccess)
    (Default|InteractwithGate _asthird_person_character self false)
    (Variables|/Game/ThirdPersonBP/Blueprints/ThirdPersonCharacter.ThirdPersonCharacter_C|SetWidgetVisible _asthird_person_character false)))

(event Custom|Close%20Gate
  (bind _staticmesh (Variables|Default|GetStaticMesh))
  (bind _relativelocation (Variables|/Script/Engine.SceneComponent|GetRelativeLocation _staticmesh))
  ;[1 1 1] Gate Close Function#
  (Utilities|FlowControl|DoOnce false
    (:Completed
      (bind _platformposition (Timeline|GateClose Play)
        (:Update
          (Transformation|SetRelativeLocation _staticmesh (Math|Vector|MakeVector (.x _relativelocation) (.y _relativelocation) _platformposition) false false))))))

(event Custom|ClosePlatform
  (bind _staticmesh (Variables|Default|GetStaticMesh))
  (bind _relativelocation (Variables|/Script/Engine.SceneComponent|GetRelativeLocation _staticmesh))
  ;[1 1 1] Gate Close Function#
  (bind _platformposition (Timeline|GateClose Reverse)
    (:Update
      (Transformation|SetRelativeLocation _staticmesh (Math|Vector|MakeVector (.x _relativelocation) (.y _relativelocation) _platformposition) false false))))

(fn ConstructionScript)